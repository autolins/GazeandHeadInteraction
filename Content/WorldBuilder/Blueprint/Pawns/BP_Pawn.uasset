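; AR head-mounted pawn that lets the user toggle gates on BP_IslandGaze actors by looking at them and blinking three times.
; It starts the AR session on play, then each tick draws a head-direction debug trace and stores the hit of an eye-gaze trace.
; Blinks are inferred from brief gaze-data dropouts and counted within a retriggerable delay window.
; The third blink passes the gazed component to ToggleGate.
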(event `self.ReceiveBeginPlay`
  (`self.PrepareForAR`))

(event `self.ReceiveEndPlay`
  (params (EndPlayReason :type "EEndPlayReason Enum" :default "Destroyed"))
  (`ARBlueprintLibrary.StopARSession`))

(event `self.ReceiveTick`
  (params (DeltaSeconds :type "Float (single-precision)"))
  (`self.HeadOrientationTracking`)
  (`self.EyeGazeTracking`))

(event `PrepareForAR`
  (`ARBlueprintLibrary.StartARSession` "/Game/WorldBuilder/Assets/AR_Session_Config.AR_Session_Config"))

(event `EyeGazeTracking`
  (bind _hmdworld_location (`self.HMDWorld location`))
  (if (`EyeTrackerFunctionLibrary.IsEyeTrackerConnected`)
    (bind (_outgazedata _returnvalue) (`EyeTrackerFunctionLibrary.GetGazeData`))
    (`self.DetectBlink` _returnvalue)
    (if _returnvalue
      (bind _outhit (`KismetSystemLibrary.LineTraceSingle` :`Start` _hmdworld_location :`End` (+ (* (`.GazeDirection` (break `EyeTrackerGazeData` _outgazedata)) 500.0) _hmdworld_location) :`TraceChannel` "TraceTypeQuery1" :`DrawDebugType` "ForOneFrame"))
      (set `self.Out Hit` _outhit))))

(event `HeadOrientationTracking`
  (bind _hmddata (`HeadMountedDisplayFunctionLibrary.GetHMDData` self))
  (if (break `XRHMDData` _hmddata)
    (bind _output_get (set `self.HMDWorld location` (`.Position` (break `XRHMDData` _hmddata))))
    (`KismetSystemLibrary.LineTraceSingle` :`Start` _output_get :`End` (+ _output_get (* (`KismetMathLibrary.GetForwardVector` (`KismetMathLibrary.Quat_Rotator` (`.Rotation` (break `XRHMDData` _hmddata)))) 500.0)) :`TraceChannel` "TraceTypeQuery1" :`DrawDebugType` "ForOneFrame" :`TraceColor` (struct :`G` 0.258975 :`B` 1.0 :`A` 1.0))))

(event `DetectBlink`
  (params (GazeTracking :type Boolean))
  (bind _blink_count (`self.Blink Count`))
  (bind _eyes_closed (`self.Eyes Closed`))
  (if GazeTracking
    (if _eyes_closed
      (set `self.Eyes Closed` false)
      (`KismetSystemLibrary.RetriggerableDelay` 0.5)
      (set `self.Blink Count` 0))
    (elif (not _eyes_closed)
      (set `self.Eyes Closed` true)
      (`KismetSystemLibrary.Delay` 0.15)
      (if (not (`self.Eyes Closed`))
        (`/Engine/EditorBlueprintResources/StandardMacros.IncrementInt` _blink_count
          (:`  `
            (if (> _blink_count 3)
              (set `self.Blink Count` 0)
              (else
                (`self.UserBlink`)))))))))

(event `UserBlink`
  (bind (_out_hit_bblockinghit _out_hit_binitialoverlap _out_hit_time _out_hit_distance _out_hit_location _out_hit_impactpoint _out_hit_normal _out_hit_impactnormal _out_hit_physmat _out_hit_hitactor _out_hit_hitcomponent) (`GameplayStatics.BreakHitResult` (`self.Out Hit`)))
  (switch `int` (`self.Blink Count`)
    (:`3`
      (bind _asbp_island_gaze (cast `/Game/WorldBuilder/Blueprint/BP_IslandGaze` _out_hit_hitactor))
      (`/Game/WorldBuilder/Blueprint/BP_IslandGaze.ToggleGate` _asbp_island_gaze _out_hit_hitcomponent))))

(fn `UserConstructionScript`)